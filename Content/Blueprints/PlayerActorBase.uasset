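; Base player actor for what appears to be an arithmetic quiz game, creating the Game widget and adding it to the viewport on BeginPlay.
; RefreshQuestion picks two small random operands and an operator, which currently always resolves to Addition, then prints the question as a string.
; CorrectAnswer and IncorrectAnswer are empty events, and the file contains no answer-checking logic.
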(event `self.ReceiveBeginPlay`
  (bind _returnvalue (`|CreateWidget` "/Game/Blueprints/Game.Game_C"))
  (`UserWidget.AddToViewport` _returnvalue 0))

(event `RefreshQuestion`
  (set `self.FirstNumber` (`KismetMathLibrary.RandomIntegerInRange` 1 5))
  (set `self.SecondNumber` (`KismetMathLibrary.RandomIntegerInRange` 1 5))
  (set `self.SelectedOperator` (select `int` (`KismetMathLibrary.RandomIntegerInRange` 0) :`0` (`self.Addition`) :`1` ""))
  (`KismetSystemLibrary.PrintString` (`KismetStringLibrary.Concat_StrStr` (`KismetStringLibrary.Conv_IntToString` (`self.FirstNumber`)) (`self.SelectedOperator`) (`KismetStringLibrary.Conv_IntToString` (`self.SecondNumber`)))))

(event `IncorrectAnswer`)

(event `CorrectAnswer`)

(fn `UserConstructionScript`)