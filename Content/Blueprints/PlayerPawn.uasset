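; Player pawn running a local two-player math duel where answers fire rifles, plus pause and game-over screens.
; Each player gets random addition or subtraction equations with three options, built through the Setoption macro, answered with A/B/C or 1/2/3.
; Correct answers damage the opponent, while wrong ones cost the answerer more health, both randomly rolled.
; SetCorrectAns2 writes to CorrectAns1, leaving CorrectAns2 unset.
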(event `InputAction|Pause`
  (params (Key :type "Key Structure" :default "AnyKey"))
  (:`Pressed`
    (if (not (`self.IsPaused`))
      (set `self.IsPaused` true)
      (bind _returnvalue (`|CreateWidget` "/Game/Blueprints/PauseMenu.PauseMenu_C"))
      (`UserWidget.AddToViewport` _returnvalue 0)
      (`Widget.RemoveFromParent` (`self.GameWidget`))
      (set `PlayerController.bShowMouseCursor` true (`GameplayStatics.GetPlayerController` 0))
      (`GameplayStatics.SetGamePaused` true))))

(event `UnPause`
  (set `self.IsPaused` false)
  (bind _returnvalue (`|CreateWidget` "/Game/Blueprints/Game.Game_C"))
  (set `self.GameWidget` _returnvalue)
  (`UserWidget.AddToViewport` _returnvalue 0)
  (`Widget.RemoveFromParent` (stale `InputAction|Pause` _returnvalue))
  (set `PlayerController.bShowMouseCursor` false (`GameplayStatics.GetPlayerController` 0))
  (`GameplayStatics.SetGamePaused` false))

(event `DamageP1Wrong`
  (if (> (`KismetMathLibrary.RandomIntegerInRange` 0 5) 4)
    (bind _output_get (set `self.PlayerOneDamage` (`KismetMathLibrary.RandomFloatInRange` 100.0 125.0)))
    (set `self.Player1Health` (- (`self.Player1Health`) _output_get))
    (set `self.PlayerOneDamage` 0.0)
    (else
      (bind _output_get_2 (set `self.PlayerOneDamage` (`KismetMathLibrary.RandomFloatInRange` 75.0 100.0)))
      (set `self.Player1Health` (- (`self.Player1Health`) _output_get_2))
      (set `self.PlayerOneDamage` 0.0)))
  (if (<= (`self.Player1Health`) 0.0)
    (`SkeletalMeshComponent.PlayAnimation` (`self.PlayerOne`) "/Game/Blueprints/Rifle_Death_3.Rifle_Death_3" false)
    (`WidgetLayoutLibrary.RemoveAllWidgets`)
    (bind _returnvalue (`|CreateWidget` "/Game/Blueprints/GameOverWidget.GameOverWidget_C"))
    (`UserWidget.AddToViewport` _returnvalue 0)
    (set `PlayerController.bShowMouseCursor` true (`GameplayStatics.GetPlayerController` 0))
    (set `self.GameOverText` "Player 1 wins")))

(event `DamageP2Wrong`
  (if (> (`KismetMathLibrary.RandomIntegerInRange` 0 5) 4)
    (bind _output_get (set `self.PlayerTwodamage` (`KismetMathLibrary.RandomFloatInRange` 100.0 125.0)))
    (set `self.Player2Health` (- (`self.Player2Health`) _output_get))
    (set `self.PlayerTwodamage` 0.0)
    (else
      (bind _output_get_2 (set `self.PlayerTwodamage` (`KismetMathLibrary.RandomFloatInRange` 75.0 100.0)))
      (set `self.Player2Health` (- (`self.Player2Health`) _output_get_2))
      (set `self.PlayerTwodamage` 0.0)))
  (if (<= (`self.Player2Health`) 0.0)
    (`SkeletalMeshComponent.PlayAnimation` (`self.PlayerTwo`) "/Game/Blueprints/Rifle_Death_3.Rifle_Death_3" false)
    (`WidgetLayoutLibrary.RemoveAllWidgets`)
    (bind _returnvalue (`|CreateWidget` "/Game/Blueprints/GameOverWidget.GameOverWidget_C"))
    (`UserWidget.AddToViewport` _returnvalue 0)
    (set `PlayerController.bShowMouseCursor` true (`GameplayStatics.GetPlayerController` 0))
    (set `self.GameOverText` "Player 2 wins")))

(event `DamagePlayerOne`
  (if (> (`KismetMathLibrary.RandomIntegerInRange` 0 5) 4)
    (bind _output_get (set `self.PlayerOneDamage` (`KismetMathLibrary.RandomFloatInRange` 50.0 75.0)))
    (set `self.Player1Health` (- (`self.Player1Health`) _output_get))
    (set `self.PlayerOneDamage` 0.0)
    (else
      (bind _output_get_2 (set `self.PlayerOneDamage` (`KismetMathLibrary.RandomFloatInRange` 25.0 50.0)))
      (set `self.Player1Health` (- (`self.Player1Health`) _output_get_2))
      (set `self.PlayerOneDamage` 0.0)))
  (if (<= (`self.Player1Health`) 0.0)
    (`SkeletalMeshComponent.PlayAnimation` (`self.PlayerOne`) "/Game/Blueprints/Rifle_Death_3.Rifle_Death_3" false)
    (`WidgetLayoutLibrary.RemoveAllWidgets`)
    (bind _returnvalue (`|CreateWidget` "/Game/Blueprints/GameOverWidget.GameOverWidget_C"))
    (`UserWidget.AddToViewport` _returnvalue 0)
    (set `PlayerController.bShowMouseCursor` true (`GameplayStatics.GetPlayerController` 0))
    (set `self.GameOverText` "Player 2 wins")))

(event `DamagePlayerTwo`
  (if (> (`KismetMathLibrary.RandomIntegerInRange` 0 5) 4)
    (bind _output_get (set `self.PlayerTwodamage` (`KismetMathLibrary.RandomFloatInRange` 50.0 75.0)))
    (set `self.Player2Health` (- (`self.Player2Health`) _output_get))
    (set `self.PlayerTwodamage` 0.0)
    (else
      (bind _output_get_2 (set `self.PlayerTwodamage` (`KismetMathLibrary.RandomFloatInRange` 25.0 50.0)))
      (set `self.Player2Health` (- (`self.Player2Health`) _output_get_2))
      (set `self.PlayerTwodamage` 0.0)))
  (if (<= (`self.Player2Health`) 0.0)
    (`SkeletalMeshComponent.PlayAnimation` (`self.PlayerTwo`) "/Game/Blueprints/Rifle_Death_3.Rifle_Death_3" false)
    (`WidgetLayoutLibrary.RemoveAllWidgets`)
    (bind _returnvalue (`|CreateWidget` "/Game/Blueprints/GameOverWidget.GameOverWidget_C"))
    (`UserWidget.AddToViewport` _returnvalue 0)
    (set `PlayerController.bShowMouseCursor` true (`GameplayStatics.GetPlayerController` 0))
    (set `self.GameOverText` "Player 1 wins")))

(event `self.ReceiveBeginPlay`
  (bind _returnvalue (`|CreateWidget` "/Game/Blueprints/Game.Game_C"))
  (set `self.GameWidget` _returnvalue)
  (`UserWidget.AddToViewport` _returnvalue 0)
  (`self.MakeNewEquation1`)
  (`self.MakeNewEquation2`))

(event `MakeNewEquation1`
  (bind _output_get (set `self.Value1_1` (`KismetMathLibrary.RandomIntegerInRange` 10 (`self.DifficultyValue`))))
  (bind _output_get_2 (set `self.Value1_2` (`KismetMathLibrary.RandomIntegerInRange` 10 (`self.DifficultyValue`))))
  (bind _output_get_3 (set `self.Operator1` (select `int` (`KismetMathLibrary.RandomIntegerInRange` 0 1) :`0` "+" :`1` "-")))
  (set `self.EquationPlayerOne` (`KismetStringLibrary.Concat_StrStr` (`KismetStringLibrary.Conv_IntToString` _output_get) _output_get_3 (`KismetStringLibrary.Conv_IntToString` _output_get_2)))
  (`self.SetGoodOption`)
  (`self.SetCorrectAns1`)
  (`self.SetA`)
  (`self.SetB`)
  (`self.SetC`))

(event `MakeNewEquation2`
  (bind _output_get (set `self.Value2_1` (`KismetMathLibrary.RandomIntegerInRange` 10 (`self.DifficultyValue`))))
  (bind _output_get_2 (set `self.Value2_2` (`KismetMathLibrary.RandomIntegerInRange` 10 (`self.DifficultyValue`))))
  (bind _output_get_3 (set `self.Operator2` (select `int` (`KismetMathLibrary.RandomIntegerInRange` 0 1) :`0` "+" :`1` "-")))
  (set `self.EquationPlayerTwo` (`KismetStringLibrary.Concat_StrStr` (`KismetStringLibrary.Conv_IntToString` _output_get) _output_get_3 (`KismetStringLibrary.Conv_IntToString` _output_get_2)))
  (`self.SetGoodOption2`)
  (`self.SetCorrectAns2`)
  (`self.Set 1`)
  (`self.Set 2`)
  (`self.Set 3`))

(event `SetA`
  ;[1 1 1] Set option a
  (if (`self.IsAGood`)
    (bind (_valaddgood _valsubgood _valaddbad _valsubbad) (`self.Setoption` (`self.Operator1`) (`self.Value1_1`) (`self.Value1_2`) :!label _label)
      (:`GoodAdd`
        (set `self.OptionA` _valaddgood))
      (:`GoodSub`
        (set `self.OptionA` _valsubgood))
      (:`BadAdd`
        (set `self.OptionA` _valaddbad))
      (:`BadSub`
        (set `self.OptionA` _valsubbad)))
    (if (`self.IsAGood`)
      _
      (elif (== (`self.OptionA`) (`self.CorrectAns1`))
        (`self.SetA`)))
    (else
      (goto _label :!via `Bad`))))

(event `SetB`
  (if (`self.IsBGood`)
    (bind (_valaddgood _valsubgood _valaddbad _valsubbad) (`self.Setoption` (`self.Operator1`) (`self.Value1_1`) (`self.Value1_2`) :!label _label_2)
      (:`GoodAdd`
        (set `self.OptionB` _valaddgood))
      (:`GoodSub`
        (set `self.OptionB` _valsubgood))
      (:`BadAdd`
        (set `self.OptionB` _valaddbad))
      (:`BadSub`
        (set `self.OptionB` _valsubbad)))
    (if (`self.IsBGood`)
      _
      (elif (== (`self.OptionB`) (`self.CorrectAns1`))
        (`self.SetB`)))
    (else
      (goto _label_2 :!via `Bad`))))

(event `SetC`
  (if (`self.IsCGood`)
    (bind (_valaddgood _valsubgood _valaddbad _valsubbad) (`self.Setoption` (`self.Operator1`) (`self.Value1_1`) (`self.Value1_2`) :!label _label_3)
      (:`GoodAdd`
        (set `self.OptionC` _valaddgood))
      (:`GoodSub`
        (set `self.OptionC` _valsubgood))
      (:`BadAdd`
        (set `self.OptionC` _valaddbad))
      (:`BadSub`
        (set `self.OptionC` _valsubbad)))
    (if (`self.IsCGood`)
      _
      (elif (== (`self.OptionC`) (`self.CorrectAns1`))
        (`self.SetC`)))
    (else
      (goto _label_3 :!via `Bad`))))

(event `InputAction|A`
  (params (Key :type "Key Structure" :default "AnyKey"))
  (:`Pressed`
    (if (`self.IsAGood`)
      (`self.MakeNewEquation1`)
      (`KismetSystemLibrary.PrintString` "CorectAnswer" true true (struct :`R` 1.0 :`A` 1.0) 5.0)
      (set `self.IsAiming` true)
      (`KismetSystemLibrary.Delay` 1.0 :!label _label_4)
      (`self.DamagePlayerTwo`)
      (`SkeletalMeshComponent.PlayAnimation` (`self.Gun`) "/Game/SciFiWeapDark/Weapons/Anims/Fire_Rifle_W.Fire_Rifle_W" false)
      (else
        (`self.MakeNewEquation1`)
        (`KismetSystemLibrary.PrintString` "Wrong Answer" true true (struct :`R` 1.0 :`A` 1.0) 5.0)
        (set `self.IsAiming` true)
        (`KismetSystemLibrary.Delay` 1.0 :!label _label_5)
        (`self.DamageP1Wrong`)
        (`SkeletalMeshComponent.PlayAnimation` (`self.Gun2`) "/Game/SciFiWeapDark/Weapons/Anims/Fire_Rifle_W.Fire_Rifle_W" false)))
    (`KismetSystemLibrary.Delay` 1.0)
    (set `self.IsAiming` false)))

(event `InputAction|B`
  (params (Key :type "Key Structure" :default "AnyKey"))
  (:`Pressed`
    (if (`self.IsBGood`)
      (`self.MakeNewEquation1`)
      (`KismetSystemLibrary.PrintString` "CorectAnswer" true true (struct :`R` 1.0 :`A` 1.0) 5.0)
      (set `self.IsAiming` true)
      (goto _label_4)
      (else
        (`self.MakeNewEquation1`)
        (`KismetSystemLibrary.PrintString` "Wrong Answer" true true (struct :`R` 1.0 :`A` 1.0) 5.0)
        (set `self.IsAiming` true)
        (goto _label_5)))))

(event `InputAction|C`
  (params (Key :type "Key Structure" :default "AnyKey"))
  (:`Pressed`
    (if (`self.IsCGood`)
      (`self.MakeNewEquation1`)
      (`KismetSystemLibrary.PrintString` "CorectAnswer" true true (struct :`R` 1.0 :`A` 1.0) 5.0)
      (set `self.IsAiming` true)
      (goto _label_4)
      (else
        (`self.MakeNewEquation1`)
        (`KismetSystemLibrary.PrintString` "Wrong Answer" true true (struct :`R` 1.0 :`A` 1.0) 5.0)
        (set `self.IsAiming` true)
        (goto _label_5)))))

(event `Set 1`
  (if (`self.Is1Good`)
    (bind (_valaddgood _valsubgood _valaddbad _valsubbad) (`self.Setoption` (`self.Operator2`) (`self.Value2_1`) (`self.Value2_2`) :!label _label_6)
      (:`GoodAdd`
        (set `self.Option1` _valaddgood))
      (:`GoodSub`
        (set `self.Option1` _valsubgood))
      (:`BadAdd`
        (set `self.Option1` _valaddbad))
      (:`BadSub`
        (set `self.Option1` _valsubbad)))
    (if (`self.Is1Good`)
      _
      (elif (== (`self.CorrectAns2`) (`self.Option1`))
        (`self.Set 1`)))
    (else
      (goto _label_6 :!via `Bad`))))

(event `Set 2`
  (if (`self.Is2Good`)
    (bind (_valaddgood _valsubgood _valaddbad _valsubbad) (`self.Setoption` (`self.Operator2`) (`self.Value2_1`) (`self.Value2_2`) :!label _label_7)
      (:`GoodAdd`
        (set `self.Option2` _valaddgood))
      (:`GoodSub`
        (set `self.Option2` _valsubgood))
      (:`BadAdd`
        (set `self.Option2` _valaddbad))
      (:`BadSub`
        (set `self.Option2` _valsubbad)))
    (if (`self.Is2Good`)
      _
      (elif (== (`self.CorrectAns2`) (`self.Option2`))
        (`self.Set 2`)))
    (else
      (goto _label_7 :!via `Bad`))))

(event `Set 3`
  (if (`self.Is3Good`)
    (bind (_valaddgood _valsubgood _valaddbad _valsubbad) (`self.Setoption` (`self.Operator2`) (`self.Value2_1`) (`self.Value2_2`) :!label _label_8)
      (:`GoodAdd`
        (set `self.Option3` _valaddgood))
      (:`GoodSub`
        (set `self.Option3` _valsubgood))
      (:`BadAdd`
        (set `self.Option3` _valaddbad))
      (:`BadSub`
        (set `self.Option3` _valsubbad)))
    (if (`self.Is3Good`)
      _
      (elif (== (`self.CorrectAns2`) (`self.Option3`))
        (`self.Set 3`)))
    (else
      (goto _label_8 :!via `Bad`))))

(event `InputAction|1`
  (params (Key :type "Key Structure" :default "AnyKey"))
  (:`Pressed`
    (if (`self.Is1Good`)
      (`self.MakeNewEquation2`)
      (set `self.IsAiming` true)
      (`KismetSystemLibrary.Delay` 1.0 :!label _label_9)
      (`self.DamagePlayerOne`)
      (`SkeletalMeshComponent.PlayAnimation` (`self.Gun2`) "/Game/SciFiWeapDark/Weapons/Anims/Fire_Rifle_W.Fire_Rifle_W" false)
      (else
        (`self.MakeNewEquation2`)
        (set `self.IsAiming` true)
        (`KismetSystemLibrary.Delay` 0.2 :!label _label_10)
        (`self.DamageP2Wrong`)
        (`SkeletalMeshComponent.PlayAnimation` (`self.Gun`) "/Game/SciFiWeapDark/Weapons/Anims/Fire_Rifle_W.Fire_Rifle_W" false)))
    (`KismetSystemLibrary.Delay` 1.0)
    (set `self.IsAiming` false)))

(event `InputAction|2`
  (params (Key :type "Key Structure" :default "AnyKey"))
  (:`Pressed`
    (if (`self.Is2Good`)
      (`self.MakeNewEquation2`)
      (set `self.IsAiming` true)
      (goto _label_9)
      (else
        (`self.MakeNewEquation2`)
        (set `self.IsAiming` true)
        (goto _label_10)))))

(event `InputAction|3`
  (params (Key :type "Key Structure" :default "AnyKey"))
  (:`Pressed`
    (if (`self.Is3Good`)
      (`self.MakeNewEquation2`)
      (set `self.IsAiming` true)
      (goto _label_9)
      (else
        (`self.MakeNewEquation2`)
        (set `self.IsAiming` true)
        (goto _label_10)))))

(fn `SetCorrectAns1`
  (if (`KismetStringLibrary.EqualEqual_StrStr` (`self.Operator1`) "+")
    (set `self.CorrectAns1` (+ (`self.Value1_1`) (`self.Value1_2`)))
    (else
      (set `self.CorrectAns1` (- (`self.Value1_1`) (`self.Value1_2`))))))

(fn `SetCorrectAns2`
  (if (`KismetStringLibrary.EqualEqual_StrStr` (`self.Operator2`) "+")
    (set `self.CorrectAns1` (+ (`self.Value2_1`) (`self.Value2_2`)))
    (else
      (set `self.CorrectAns1` (- (`self.Value2_1`) (`self.Value2_2`))))))

(fn `SetGoodOption`
  (locals (IntValue :type Integer))
  (set `local.IntValue` (`KismetMathLibrary.RandomIntegerInRange` 1 3))
  (if (== (`local.IntValue`) 1)
    (set `self.IsAGood` true)
    (set `self.IsBGood` false)
    (set `self.IsCGood` false)
    (elif (== (`local.IntValue`) 2)
      (set `self.IsBGood` true)
      (set `self.IsAGood` false)
      (set `self.IsCGood` false)
      (else
        (set `self.IsCGood` true)
        (set `self.IsAGood` false)
        (set `self.IsBGood` false)))))

(fn `SetGoodOption2`
  (locals (IntValue :type Integer))
  (set `local.IntValue` (`KismetMathLibrary.RandomIntegerInRange` 1 3))
  (if (== (`local.IntValue`) 1)
    (set `self.Is1Good` true)
    (set `self.Is2Good` false)
    (set `self.Is3Good` false)
    (elif (== (`local.IntValue`) 2)
      (set `self.Is1Good` false)
      (set `self.Is2Good` true)
      (set `self.Is3Good` false)
      (else
        (set `self.Is1Good` false)
        (set `self.Is2Good` false)
        (set `self.Is3Good` true)))))

(fn `UserConstructionScript`)